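; FloorColisionBox is a trigger volume that catches pickups and cards overlapping it and teleports them back to the height of its Billboard marker.
; On box overlap, a BP_MainPickUp or FGCard keeps its X and Y but takes the billboard's Z, with rotation reset.
; Pickups also have their linear velocity zeroed and their component rotation leveled to yaw only.
; An angular velocity reset exists but is not connected.
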(event OnComponentBeginOverlap(Box)
  (params (OverlappedComponent :type Primitive%20Component%20Object%20Reference) (OtherActor :type Actor%20Object%20Reference) (OtherComp :type Primitive%20Component%20Object%20Reference) (OtherBodyIndex :type Integer) (bFromSweep :type Boolean) (SweepResult :type Hit%20Result%20Structure%20%28by%20ref%29))
  (bind _returnvalue (Transformation|GetActorLocation OtherActor))
  (bind _billboard (Variables|Default|GetBillboard))
  (bind _returnvalue_2 (Transformation|GetWorldLocation _billboard))
  (bind (_x _y) (Math|Vector|BreakVector _returnvalue))
  (bind _z (Math|Vector|BreakVector _returnvalue_2))
  (bind _returnvalue_3 (Math|Vector|MakeVector _x _y _z))
  (bind _asbp_main_pick_up (Utilities|Casting|CastToBP_MainPickUp OtherActor)
    (:then
      (Transformation|Teleport _asbp_main_pick_up _returnvalue_3 "0, 0, 0")
      (Physics|SetPhysicsLinearVelocity OtherComp "0, 0, 0" false "None")
      (Transformation|SetWorldRotation OtherComp (Math|Rotator|MakeRotator 0.0 0.0 (.Yaw (Math|Rotator|BreakRotator (Transformation|GetActorRotation OtherActor)))) false false))
    (:CastFailed
      (bind _asfgcard (Utilities|Casting|CastToFGCard OtherActor))
      (Transformation|Teleport _asfgcard _returnvalue_3 "0, 0, 0"))))

(event EventBeginPlay)

(event Collision|EventActorBeginOverlap
  (params (OtherActor :type Actor%20Object%20Reference)))

(event EventTick
  (params (DeltaSeconds :type Float%20%28single-precision%29)))

(fn ConstructionScript)