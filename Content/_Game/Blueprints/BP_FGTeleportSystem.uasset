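; BP_FGTeleportSystem is a teleporter Blueprint that handles what happens when a teleport occurs; the teleport itself is not performed in this graph.
; OnTeleport can disable overlap events on TeleportBounds, making the teleporter one-shot when TurnOfAfterTeleport is set.
; If glitching is enabled, it switches on a post-process glitch through a Material Parameter Collection scalar, then switches it off after a configurable delay.
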(event EventBeginPlay)

(event Collision|EventActorBeginOverlap
  (params (OtherActor :type Actor%20Object%20Reference)))

(event EventTick
  (params (DeltaSeconds :type Float%20%28single-precision%29)))

(event EventOnTeleport
  (if (Variables|Default|GetTurnOfAfterTeleport)
    (Variables|/Script/Engine.PrimitiveComponent|SetbGenerateOverlapEvents (Variables|Default|GetTeleportBounds) false))
  (if (Variables|Default|GetShouldGlitchWhenTeleporting)
    (Rendering|Material|SetScalarParameterValue (Variables|Default|GetGlitch%20Material%20Collection) (Utilities|String|StringToName "Glitch_PP_Switch") 1.0 :!class /Script/Engine.KismetMaterialLibrary)
    (Utilities|FlowControl|Delay (Variables|Default|GetLengthOfGlitch))
    (Rendering|Material|SetScalarParameterValue (Variables|Default|GetGlitch%20Material%20Collection) (Utilities|String|StringToName "Glitch_PP_Switch") 0.0 :!class /Script/Engine.KismetMaterialLibrary)))

(fn ConstructionScript)