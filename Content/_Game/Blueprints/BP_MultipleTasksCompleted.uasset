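; BP_MultipleTasksCompleted counts completed tasks and triggers voicelines at progress milestones.
; On BeginPlay it binds one shared event to the completion delegate of each entry in TaskHandlers and caches BP_GameMode inside that loop.
; Each completion increments a counter, and two hardcoded counts each play a specific voiceline through the game mode after a short delay.
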(event Custom|OnCompleteTaskDelegate_Event
  (bind _output_get (Variables|Default|SetNumberOfTasksCompleted (+ (Variables|Default|GetNumberOfTasksCompleted) 1)))
  (switch int _output_get
    (:4
      (Utilities|FlowControl|Delay 1.0)
      (Default|PlayVoiceline (stale EventBeginPlay _asbp_game_mode) 6))
    (:6
      (Utilities|FlowControl|Delay 1.0)
      (Default|PlayVoiceline (stale EventBeginPlay _asbp_game_mode) 11))))

(event EventBeginPlay
  (for _array_element (Variables|Default|GetTaskHandlers)
    (EventDispatchers|AssignOnCompleteTaskDelegate _array_element (delegate Custom|OnCompleteTaskDelegate_Event))
    (bind _asbp_game_mode (Utilities|Casting|CastToBP_GameMode (Game|GetGameMode)))))

(fn ConstructionScript)