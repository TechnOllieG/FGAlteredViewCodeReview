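; BP_CleanDeskTask is a task that completes when desk areas are clear of interactable actors, then plays a voiceline once through BP_GameMode.
; Every Tick, it runs component overlap queries on AreaToClean and AreaToClean2, proceeding only when both find no FGInteractable.
; A third query on AreaToClean1 looks for FGPickupInteractable, but its result is ignored.
; CompleteTaskComponent sits before the DoOnce, so it repeats each frame while those areas stay clear.
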(event EventTick
  (params (DeltaSeconds :type Float%20%28single-precision%29))
  (bind _areatoclean (Variables|Default|GetAreaToClean))
  (bind _areatoclean2 (Variables|Default|GetAreaToClean2))
  (bind _areatoclean1 (Variables|Default|GetAreaToClean1))
  (bind _returnvalue (Collision|ComponentOverlapActors _areatoclean (Transformation|GetWorldTransform _areatoclean) (Utilities|Array|MakeArray "ObjectTypeQuery2") "/Script/GP3_Team02.FGInteractable"))
  (if (not _returnvalue)
    (bind _returnvalue_2 (Collision|ComponentOverlapActors _areatoclean2 (Transformation|GetWorldTransform _areatoclean2) (Utilities|Array|MakeArray "ObjectTypeQuery2") "/Script/GP3_Team02.FGInteractable"))
    (if (not _returnvalue_2)
      (Collision|ComponentOverlapActors _areatoclean1 (Transformation|GetWorldTransform _areatoclean1) (Utilities|Array|MakeArray "ObjectTypeQuery2") "/Script/GP3_Team02.FGPickupInteractable")
      (Class|FGTaskComponent|CompleteTaskComponent (Variables|Default|GetFGTask))
      (Utilities|FlowControl|DoOnce false
        (:Completed
          (bind _asbp_game_mode (Utilities|Casting|CastToBP_GameMode (Game|GetGameMode)))
          (Default|PlayVoiceline _asbp_game_mode 14))))))

(fn ConstructionScript)