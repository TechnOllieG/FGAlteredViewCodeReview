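; BP_Shredder is an office shredder task actor that reacts to items overlapping its Box, playing Niagara effects and mostly a shredder audio event.
; When inactive or fed a tablet, it only shows a broken effect.
; Shredable folders are destroyed and counted, with the fourth completing the FGTask and playing a voiceline.
; Key cards teleport to SpawnPoint, puzzle folders respawn there when the last is shredded, and other pickups are destroyed.
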(event OnComponentBeginOverlap(Box)
  (params (OverlappedComponent :type Primitive%20Component%20Object%20Reference) (OtherActor :type Actor%20Object%20Reference) (OtherComp :type Primitive%20Component%20Object%20Reference) (OtherBodyIndex :type Integer) (bFromSweep :type Boolean) (SweepResult :type Hit%20Result%20Structure%20%28by%20ref%29))
  (bind _box (Variables|Default|GetBox))
  (bind _box_2 (Variables|Default|GetBox))
  (bind _box_3 (Variables|Default|GetBox))
  (bind _brokenvfx (Variables|Default|GetBrokenVFX))
  (bind _returnvalue (Transformation|GetWorldLocation _box_2))
  (bind _returnvalue_2 (Transformation|GetWorldRotation _box_2))
  (if (Variables|Default|GetIs%20active)
    (Utilities|Casting|CastToBP_Tablet OtherActor
      (:then
        (Niagara|SpawnSystematLocation "/Game/_Game/Assets/VFX/NiagaraSystems/NS_BrokenShredder.NS_BrokenShredder" (Transformation|GetWorldLocation _brokenvfx) (Transformation|GetWorldRotation _brokenvfx) :!label _label))
      (:CastFailed
        (Utilities|Casting|CastToBP_ShreddableInt OtherActor
          (:then
            (Development|PrintString "notkeycard")
            (Niagara|SpawnSystematLocation "/Game/_Game/Assets/VFX/NiagaraSystems/NS_Shredder.NS_Shredder" (Transformation|GetWorldLocation _box) (Transformation|GetWorldRotation _box))
            (Utilities|Casting|CastToBP_Shredable_Folder OtherActor)
            (Variables|Default|SetTimes%20Shredded (+ (Variables|Default|GetTimes%20Shredded) 1))
            (Actor|DestroyActor OtherActor)
            (if (== (Variables|Default|GetTimes%20Shredded) 4)
              (Class|FGTaskComponent|CompleteTaskComponent (Variables|Default|GetFGTask))
              (bind _asbp_game_mode (Utilities|Casting|CastToBP_GameMode (Game|GetGameMode)))
              (Default|PlayVoiceline _asbp_game_mode 5))
            (Class|FMODBlueprintStatics|PlayEventatLocation "/Game/FMOD/Events/Interactables/Shredder.Shredder" (Math|Conversions|ToTransform(Vector) (Transformation|GetActorLocation)) :!label _label_2))
          (:CastFailed
            (Utilities|Casting|CastToBP_FGCard OtherActor
              (:then
                (Development|PrintString "Destroy")
                (Niagara|SpawnSystematLocation "/Game/_Game/Assets/VFX/NiagaraSystems/NS_Shredder.NS_Shredder" (Transformation|GetWorldLocation _box_3) (Transformation|GetWorldRotation _box_3))
                (CallFunction|SpawnKeyCard))
              (:CastFailed
                (bind _asbp_pickupable_puzzle_folder (Utilities|Casting|CastToBP_Pickupable_PuzzleFolder OtherActor)
                  (:then
                    (Development|PrintString "Hello")
                    (Niagara|SpawnSystematLocation "/Game/_Game/Assets/VFX/NiagaraSystems/NS_Shredder.NS_Shredder" _returnvalue _returnvalue_2)
                    (Actor|DestroyActor _asbp_pickupable_puzzle_folder)
                    (Audio|PlaySoundatLocation "/Engine/VREditor/Sounds/UI/Drop_Item_From_ContentBrowser.Drop_Item_From_ContentBrowser" "0, 0, 0" "0, 0, 0" 1.0 1.0 0.0 0 0 0)
                    (bind _outactors (Actor|GetAllActorsOfClass "/Game/_Game/Blueprints/Task_BP/BP_Pickupable_PuzzleFolder.BP_Pickupable_PuzzleFolder_C"))
                    (if (== (Utilities|Array|Length _outactors) 1)
                      (Game|SpawnActorfromClass "/Game/_Game/Blueprints/Task_BP/BP_Pickupable_PuzzleFolder.BP_Pickupable_PuzzleFolder_C" (Transformation|GetWorldTransform (Variables|Default|GetSpawnPoint)) "Undefined" 0 0)
                      (goto _label_2)))
                  (:CastFailed
                    (bind _asfgpickup_interactable (Utilities|Casting|CastToFGPickupInteractable OtherActor))
                    (Development|PrintString "yolo")
                    (Niagara|SpawnSystematLocation "/Game/_Game/Assets/VFX/NiagaraSystems/NS_Shredder.NS_Shredder" _returnvalue _returnvalue_2)
                    (Actor|DestroyActor _asfgpickup_interactable)
                    (goto _label_2)))))))))
    (else
      (goto _label))))

(event Custom|SpawnKeyCard
  (bind _spawnpoint (Variables|Default|GetSpawnPoint))
  (bind _returnvalue (Transformation|GetWorldLocation _spawnpoint))
  (Transformation|Teleport (stale OnComponentBeginOverlap(Box) OtherActor) _returnvalue (Transformation|GetWorldRotation _spawnpoint))
  (Audio|PlaySoundatLocation "/Engine/VREditor/Sounds/UI/Drop_Item_From_ContentBrowser.Drop_Item_From_ContentBrowser" _returnvalue "0, 0, 0" 1.0 1.0 0.0 0 0 0))

(event Custom|SpawnPuzzleFolder)

(fn ConstructionScript)