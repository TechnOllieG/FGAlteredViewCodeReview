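; Task handler for the "CrainDoor" task that opens a door and swaps active teleporters when the task completes.
; On completion it destroys its verification overlap box actors, then opens the referenced card scanner door.
; It then destroys the first two teleporters and sets the bounds of the other two to overlap collision.
; Each step relies on a cast, so a failed one halts what follows, except between the last two teleporters.
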(event EventOnCompleteTask
  (for _array_element (Variables|Default|GetActorVerificationOverlapBoxes)
    (Actor|DestroyActor _array_element))
  (bind _asbp_fgcard_scanner (Utilities|Casting|CastToBP_FGCardScanner (Variables|Default|GetDoorReal)))
  (Class|FGCardScanner|OpenDoor _asbp_fgcard_scanner)
  (bind _asbp_fgteleport_system (Utilities|Casting|CastToBP_FGTeleportSystem (Variables|Default|GetTeleporter1)))
  (Actor|DestroyActor _asbp_fgteleport_system)
  (bind _asbp_fgteleport_system_2 (Utilities|Casting|CastToBP_FGTeleportSystem (Variables|Default|GetTeleporter2)))
  (Actor|DestroyActor _asbp_fgteleport_system_2)
  (Utilities|FlowControl|Sequence
    (:then_0
      (bind _asbp_fgteleport_system_3 (Utilities|Casting|CastToBP_FGTeleportSystem (Variables|Default|GetTeleporter3)))
      (Collision|SetCollisionProfileName (Variables|/Script/GP3_Team02.FGTeleportSystem|GetTeleportBounds _asbp_fgteleport_system_3) "OverlapAllDynamic" true :!class /Script/Engine.PrimitiveComponent))
    (:then_1
      (bind _asbp_fgteleport_system_4 (Utilities|Casting|CastToBP_FGTeleportSystem (Variables|Default|GetTeleporter4)))
      (Collision|SetCollisionProfileName (Variables|/Script/GP3_Team02.FGTeleportSystem|GetTeleportBounds _asbp_fgteleport_system_4) "OverlapAllDynamic" true :!class /Script/Engine.PrimitiveComponent))))

(fn ConstructionScript)