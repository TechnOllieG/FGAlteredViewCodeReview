(event EventBeginPlay
  (Rendering|SetRenderCustomDepth (Variables|Default|GetScreen) false))

(event EventInteract
  (Class|FGTaskComponent|CompleteTaskComponent (Variables|Default|GetTaskComponent))
  (Rendering|SetVisibility (Variables|Default|GetOpenMail) true false)
  (Rendering|SetVisibility (Variables|Default|GetYou'veGotMail) false false)
  (Utilities|FlowControl|DoOnce false
    (:Completed
      (bind _asbp_game_mode (Utilities|Casting|CastToBP_GameMode (Game|GetGameMode)))
      (Default|PlayVoiceline _asbp_game_mode 19))))

(fn ConstructionScript)