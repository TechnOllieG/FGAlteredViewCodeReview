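; Interactable computer task where the player opens an email screen, then sends it.
; A non-looping MultiGate steps through two interactions: the first shows the email, the second shows the sent screen, plays a sound and completes the TaskComponent.
; Sending also finds BP_ComputerScreenTaskGetEmail1 actors among FGInteractables, making them interactable and revealing their mail notice and light, with a delayed received sound.
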(event EventBeginPlay
  (Rendering|SetRenderCustomDepth (Variables|Default|GetScreen) false))

(event EventInteract
  (Utilities|FlowControl|MultiGate false false -1
    (:Out%200
      (Rendering|SetVisibility (Variables|Default|GetE-mailScreen) true false))
    (:Out%201
      (Rendering|SetVisibility (Variables|Default|GetE-mailSent) true false)
      (Class|FMODBlueprintStatics|PlayEventatLocation "/Game/FMOD/Events/Interactables/Email/Email_Sent.Email_Sent" (Math|Conversions|ToTransform(Vector) (Transformation|GetActorLocation)))
      (Rendering|SetVisibility (Variables|Default|GetE-mailScreen) false false)
      (Class|FGTaskComponent|CompleteTaskComponent (Variables|Default|GetTaskComponent))
      (bind _outactors (Actor|GetAllActorsOfClass "/Script/GP3_Team02.FGInteractable"))
      (for _array_element _outactors
        (bind _asbp_computer_screen_task_get_email_1 (Utilities|Casting|CastToBP_ComputerScreenTaskGetEmail1 _array_element))
        (Variables|/Script/GP3_Team02.FGInteractable|SetCurrentlyInteractable _asbp_computer_screen_task_get_email_1 true)
        (Rendering|SetVisibility (Variables|/Game/_Game/Blueprints/Task_BP/BP_ComputerScreenTaskGetEmail1.BP_ComputerScreenTaskGetEmail1_C|GetYou'veGotMail _asbp_computer_screen_task_get_email_1) true false)
        (Rendering|SetVisibility (Variables|/Game/_Game/Blueprints/Task_BP/BP_ComputerScreenTaskGetEmail1.BP_ComputerScreenTaskGetEmail1_C|GetRectLight _asbp_computer_screen_task_get_email_1) true false)
        (Utilities|FlowControl|Delay 2.0)
        (Class|FMODBlueprintStatics|PlayEventatLocation "/Game/FMOD/Events/Interactables/Email/Email_Received.Email_Received" (Math|Conversions|ToTransform(Vector) (Transformation|GetActorLocation _asbp_computer_screen_task_get_email_1)))))))

(fn ConstructionScript)