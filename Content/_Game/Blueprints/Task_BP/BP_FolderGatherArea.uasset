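; BP_FolderGatherArea is a task trigger area that counts puzzle folders brought into it.
; On overlap, each BP_Pickupable_PuzzleFolder not yet gathered is flagged and increments the count, as long as the task is incomplete.
; When the count equals FoldersToGather, it completes the FGTask component and teleports LabCardObject to the CardSpawnLocation position as the reward.
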(event Collision|EventActorBeginOverlap
  (params (OtherActor :type Actor%20Object%20Reference))
  (if (not (Variables|Default|GetTaskCompleted))
    (bind _asbp_pickupable_puzzle_folder (Utilities|Casting|CastToBP_Pickupable_PuzzleFolder OtherActor))
    (if (not (Variables|/Game/_Game/Blueprints/Task_BP/BP_Pickupable_PuzzleFolder.BP_Pickupable_PuzzleFolder_C|GetIsGathered _asbp_pickupable_puzzle_folder))
      (bind _output_get (Variables|Default|SetFoldersGathered (+ (Variables|Default|GetFoldersGathered) 1)))
      (Variables|/Game/_Game/Blueprints/Task_BP/BP_Pickupable_PuzzleFolder.BP_Pickupable_PuzzleFolder_C|SetIsGathered _asbp_pickupable_puzzle_folder true)
      (Math|Integer|CompareInt _output_get (Variables|Default|GetFoldersToGather)
        (:==
          (Class|FGTaskComponent|CompleteTaskComponent (Variables|Default|GetFGTask))
          (Transformation|Teleport (Variables|Default|GetLabCardObject) (Transformation|GetWorldLocation (Variables|Default|GetCardSpawnLocation)) "0, 0, 0"))))))

(fn ConstructionScript)