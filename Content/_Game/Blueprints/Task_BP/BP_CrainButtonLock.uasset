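; BP_CrainButtonLock is a task button that is triggered when a crane pickupable object enters its hit area.
; On overlap with a BP_CrainPickUpable, it plays a click sound at the button and completes its task component.
; It then tells the crane minimap widget on the game state that this button is active.
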(event OnComponentBeginOverlap(Hitarea)
  (params (OverlappedComponent :type Primitive%20Component%20Object%20Reference) (OtherActor :type Actor%20Object%20Reference) (OtherComp :type Primitive%20Component%20Object%20Reference) (OtherBodyIndex :type Integer) (bFromSweep :type Boolean) (SweepResult :type Hit%20Result%20Structure%20%28by%20ref%29))
  (Utilities|Casting|CastToBP_CrainPickUpable OtherActor)
  (Audio|PlaySoundatLocation "/Engine/VREditor/Sounds/UI/Click_on_Button.Click_on_Button" (Transformation|GetWorldLocation (Variables|Default|GetButtonarea)) "0, 0, 0" 1.0 1.0 0.0 0 0 0)
  (Class|FGTaskComponent|CompleteTaskComponent (Variables|Default|GetFGTask))
  (bind _asfggame_state_base (Utilities|Casting|CastToFGGameStateBase (Game|GetGameState)))
  (Class|FGCrainMinimapWidget|SetButtonState (Variables|/Script/GP3_Team02.FGGameStateBase|GetCrainMinimapWidget _asfggame_state_base) self true))

(fn ConstructionScript)