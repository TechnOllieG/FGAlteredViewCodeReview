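; BP_Lever is an interactable task lever that switches on a crane.
; Interact plays a timeline that pitches the lever mesh.
; Its first update, gated by DoOnce and a game mode cast, plays an FMOD pull sound, completes the task component, sets the crane's CrainOn flag and snaps a second lever actor to a fixed rotation.
; When the timeline finishes, it destroys the BlackScreen actor.
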(event EventBeginPlay)

(event Collision|EventActorBeginOverlap
  (params (OtherActor :type Actor%20Object%20Reference)))

(event EventTick
  (params (DeltaSeconds :type Float%20%28single-precision%29)))

(event EventInteract
  (bind _staticmesh (Variables|Default|GetStaticMesh))
  (bind _returnvalue (Transformation|GetWorldRotation _staticmesh))
  (bind _leverspeed (Timeline|LeverSpeed Play)
    (:Update
      (Transformation|SetWorldRotation (Variables|Default|GetStaticMesh) (Math|Rotator|MakeRotator (.roll _returnvalue) (* _leverspeed -6e+01) (.yaw _returnvalue)) false false)
      (Utilities|FlowControl|DoOnce false
        (:Completed
          (Utilities|Casting|CastToBP_GameMode (Game|GetGameMode))
          (Class|FMODBlueprintStatics|PlayEventatLocation "/Game/FMOD/Events/Interactables/Level_Pull.Level_Pull" (Math|Conversions|ToTransform(Vector) (Transformation|GetActorLocation)))
          (Class|FGTaskComponent|CompleteTaskComponent (Variables|Default|GetTaskComponent))
          (bind _asbp_crain_actor (Utilities|Casting|CastToBP_CrainActor (Variables|Default|GetCraneObject)))
          (Variables|/Script/GP3_Team02.CrainActor|SetCrainOn _asbp_crain_actor true)
          (Transformation|SetActorRotation (Variables|Default|GetExtraLever) "0,-90.000000, 0"))))
    (:Finished
      (Actor|DestroyActor (Variables|Default|GetBlackScreen)))))

(fn ConstructionScript)