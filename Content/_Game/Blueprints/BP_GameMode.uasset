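; Game mode Blueprint that plays queued voicelines one at a time as 2D audio events, with matching subtitles.
; PlayVoiceline appends an index to the queue, and that index looks up parallel arrays of events, subtitle texts and lengths.
; Tick polls the queue, using a busy flag and a Delay of the line's length before removing it.
; Subtitles receive extra display time beyond the audio length.
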(event EventTick
  (params (DeltaSeconds :type Float%20%28single-precision%29))
  (bind _length_of_voicelines (Variables|Default|GetLength%20of%20Voicelines))
  (bind _voicelines_queue (Variables|Default|GetVoicelines%20Queue))
  (bind _output (Utilities|Array|Get(acopy) _voicelines_queue))
  (bind _output_2 (Utilities|Array|Get(acopy) _length_of_voicelines _output))
  (if (> (Utilities|Array|Length (Variables|Default|GetVoicelines%20Queue)) 0)
    (if (Variables|Default|GetNot%20Ocupied)
      (Variables|Default|SetNot%20Ocupied false)
      (Class|FMODBlueprintStatics|PlayEvent2D (Utilities|Array|Get(acopy) (Variables|Default|GetVoicelines) _output))
      (Class|FGSubtitleLibrary|DisplaySubtitles (Utilities|Array|Get(acopy) (Variables|Default|GetSubtitles%20Text) _output) (+ (Variables|Default|GetSubtitle%20Extra%20Duration) _output_2))
      (Utilities|FlowControl|Delay _output_2)
      (Utilities|Array|RemoveIndex (Variables|Default|GetVoicelines%20Queue))
      (Variables|Default|SetNot%20Ocupied true))))

(fn ConstructionScript)

(fn PlayVoiceline
  (params (VoicelineIndex :type Integer))
  (Utilities|Array|Add (Variables|Default|GetVoicelines%20Queue) VoicelineIndex))