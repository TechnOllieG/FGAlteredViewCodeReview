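; Player Blueprint that handles surface-based footstep sounds, crosshair interaction feedback and a tablet doubling as task display and menu.
; Tick lerps the tablet toward its hidden, Tab-raised or menu position.
; The menu opens at BeginPlay or via Escape, blocking movement, hiding the crosshair and applying depth-of-field blur.
; While the cursor shows, a WidgetInteraction component follows the deprojected mouse ray, forwarding clicks to widgets.
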(event BPonInteractableFeedback(LineTraceComponent)
  (params (RelevantInteractable :type FG%20Interactable%20Object%20Reference) (FeedbackState :type Boolean))
  ;[1 1 1] Changing color of crosshair
  (bind _asbp_fghud (Utilities|Casting|CastToBP_FGHUD (HUD|GetHUD (Game|GetPlayerController 0))))
  (bind _aswbp_fgviewport_widget (Utilities|Casting|CastToWBP_FGViewportWidget (Variables|/Script/GP3_Team02.FGHUD|GetViewportWidget _asbp_fghud)))
  (Default|SetCrosshairFeedback _aswbp_fgviewport_widget FeedbackState))

(event EventOnStopWalking
  ;[1 1 1] Footstep sound
  (Variables|Default|SetWalking false)
  (Utilities|FlowControl|Delay 0.5)
  (Variables|Default|SetFootsteps%20Cooldown true))

(event EventOnStartWalking
  (bind _mesh (Variables|Character|GetMesh))
  (bind _returnvalue (Transformation|GetWorldLocation _mesh))
  ;[1 1 1] Footstep sound
  (Variables|Default|SetWalking true)
  (if (Variables|Default|GetFootsteps%20Cooldown)
    (Variables|Default|SetFootsteps%20Cooldown false)
    (if (Variables|Default|GetWalking) :!label _label
      (bind (_outhit _returnvalue_2) (Collision|LineTraceByChannel _returnvalue (- _returnvalue "0, 0,100.000000") "TraceTypeQuery2" false (Utilities|Array|MakeArray self) "None"))
      (if _returnvalue_2
        (switch Utilities|FlowControl|Switch|SwitchonEPhysicalSurface (Variables|/Script/PhysicsCore.PhysicalMaterial|GetSurfaceType (.PhysMat (Collision|BreakHitResult _outhit)))
          (:SurfaceType1
            (Class|FMODBlueprintStatics|PlayEvent2D "/Game/FMOD/Events/Character/Footsteps_Wood.Footsteps_Wood"))
          (:SurfaceType2
            (Class|FMODBlueprintStatics|PlayEvent2D "/Game/FMOD/Events/Character/Footsteps_Marble.Footsteps_Marble"))
          (:SurfaceType3
            (Class|FMODBlueprintStatics|PlayEvent2D "/Game/FMOD/Events/Character/Footsteps_Metal.Footsteps_Metal")))
        (Utilities|FlowControl|Delay 0.5)
        (goto _label)))))

(event EventBeginPlay
  ;[1 1 1] UI Show/Hide
  (bind _output_get (Variables|Default|SetUIStartPos (Variables|/Script/Engine.SceneComponent|GetRelativeLocation (Variables|Default|GetBP_FGTaskTablet))))
  (Variables|Default|SetUIDestinationPos (+ _output_get (* "0, 0,1.000000" (Variables|Default|GetUIUpDistance))))
  (Variables|Default|SetTargetPosition _output_get)
  ;[1 1 1] Menu Interaction Logic
  (Transformation|SetRelativeLocation (Variables|Default|GetBP_FGTaskTablet) (Variables|Default|GetTabletMenuPos) false false)
  (CallFunction|ShowMenu))

(event EventTick
  (params (DeltaSeconds :type Float%20%28single-precision%29))
  (bind _returnvalue (Game|GetPlayerController 0))
  (bind _widgetinteraction (Variables|Default|GetWidgetInteraction))
  (bind (_worldlocation _worlddirection) (Game|Player|ConvertMouseLocationToWorldSpace _returnvalue))
  ;[1 1 1] UI Show/Hide
  (if (Variables|Default|GetMenuIsUp)
    ;[1 1 1] Menu Interaction Logic
    (Transformation|SetRelativeLocation (Variables|Default|GetBP_FGTaskTablet) (Math|Vector|Lerp(Vector) (Variables|/Script/Engine.SceneComponent|GetRelativeLocation (Variables|Default|GetBP_FGTaskTablet)) (Variables|Default|GetTabletMenuPos) 0.1) false false)
    (else
      (Transformation|SetRelativeLocation (Variables|Default|GetBP_FGTaskTablet) (Math|Vector|Lerp(Vector) (Variables|/Script/Engine.SceneComponent|GetRelativeLocation (Variables|Default|GetBP_FGTaskTablet)) (Variables|Default|GetTargetPosition) 0.1) false false)))
  (if (Variables|/Script/Engine.PlayerController|GetbShowMouseCursor _returnvalue)
    (Transformation|SetWorldLocation _widgetinteraction _worldlocation false false)
    (Transformation|SetWorldRotation _widgetinteraction (Math|Rotator|MakeRotfromX _worlddirection) false false)))

(event Input|KeyboardEvents|Tab
  (params (Key :type Key%20Structure :default "None"))
  ;[1 1 1] UI Show/Hide
  (:Pressed
    (Variables|Default|SetTargetPosition (Variables|Default|GetUIDestinationPos))
    (Rendering|Components|TextRender|SetText (Variables|/Game/_Game/Blueprints/UI/WBP_UI_Tablet.WBP_UI_Tablet_C|GetTabText (CallFunction|GetTablet)) "Release tab to hide"))
  (:Released
    (Variables|Default|SetTargetPosition (Variables|Default|GetUIStartPos))
    (Rendering|Components|TextRender|SetText (Variables|/Game/_Game/Blueprints/UI/WBP_UI_Tablet.WBP_UI_Tablet_C|GetTabText (CallFunction|GetTablet)) "Hold tab to show")))

(event Input|MouseEvents|LeftMouseButton
  (params (Key :type Key%20Structure :default "None"))
  (bind _returnvalue (Game|GetPlayerController 0))
  (bind _widgetinteraction (Variables|Default|GetWidgetInteraction))
  (bind _bshowmousecursor (Variables|/Script/Engine.PlayerController|GetbShowMouseCursor _returnvalue))
  ;[1 1 1] Menu Interaction Logic
  (:Pressed
    (if _bshowmousecursor
      (Class|WidgetInteractionComponent|PressPointerKey _widgetinteraction Key)))
  (:Released
    (if _bshowmousecursor
      (Class|WidgetInteractionComponent|ReleasePointerKey _widgetinteraction Key))))

(event Input|KeyboardEvents|Escape
  (params (Key :type Key%20Structure :default "None"))
  ;[1 1 1] Menu Interaction Logic
  (:Pressed
    (if (Variables|Default|GetMenuIsUp)
      (Default|CallOnHideMenuDelegate)
      (else
        (Default|CallOnShowMenuDelegate)
        (CallFunction|ShowMenu)))))

(fn ConstructionScript)

(fn OnPressPlay
  (CallFunction|HideMenu))

(fn ShowMenu
  (bind _returnvalue (Game|GetPlayerController 0))
  (Variables|/Script/Engine.PlayerController|SetbShowMouseCursor _returnvalue true)
  (Input|SetIgnoreMoveInput _returnvalue true)
  (Variables|Default|SetMenuIsUp true)
  (bind _asbp_fghud (Utilities|Casting|CastToBP_FGHUD (HUD|GetHUD _returnvalue)))
  (bind _aswbp_fgviewport_widget (Utilities|Casting|CastToWBP_FGViewportWidget (Variables|/Script/GP3_Team02.FGHUD|GetViewportWidget _asbp_fghud)))
  (Widget|SetVisibility (Variables|/Game/_Game/Blueprints/UI/WBP_FGViewportWidget.WBP_FGViewportWidget_C|GetCrosshair _aswbp_fgviewport_widget) "Hidden")
  (Widget|SetVisibility (Variables|/Game/_Game/Blueprints/UI/WBP_UI_Tablet.WBP_UI_Tablet_C|GetTabText (CallFunction|GetTablet)) "Hidden")
  (Variables|/Script/Engine.CameraComponent|SetPostProcessSettings (Variables|Default|GetCamera) (Utilities|Struct|MakePostProcessSettings (.x (Variables|Default|GetTabletMenuPos)) 2e+01)))

(fn HideMenu
  (bind _returnvalue (Game|GetPlayerController 0))
  (Variables|/Script/Engine.PlayerController|SetbShowMouseCursor _returnvalue false)
  (Input|SetIgnoreMoveInput _returnvalue false)
  (Variables|Default|SetMenuIsUp false)
  (bind _asbp_fghud (Utilities|Casting|CastToBP_FGHUD (HUD|GetHUD _returnvalue)))
  (bind _aswbp_fgviewport_widget (Utilities|Casting|CastToWBP_FGViewportWidget (Variables|/Script/GP3_Team02.FGHUD|GetViewportWidget _asbp_fghud)))
  (Widget|SetVisibility (Variables|/Game/_Game/Blueprints/UI/WBP_FGViewportWidget.WBP_FGViewportWidget_C|GetCrosshair _aswbp_fgviewport_widget) "Visible")
  (Widget|SetVisibility (Variables|/Game/_Game/Blueprints/UI/WBP_UI_Tablet.WBP_UI_Tablet_C|GetTabText (CallFunction|GetTablet)) "Visible")
  (Variables|/Script/Engine.CameraComponent|SetPostProcessSettings (Variables|Default|GetCamera) (Utilities|Struct|MakePostProcessSettings 0.0)))

(fn GetTablet
  (if (== (Variables|Default|GetAs%20WBP%20UI%20Tablet) 0)
    (bind _asfggame_state_base (Utilities|Casting|CastToFGGameStateBase (Game|GetGameState)))
    (bind _returnvalue (Class|FGGameStateBase|GetTaskTablet _asfggame_state_base))
    (bind _aswbp_ui_tablet (Utilities|Casting|CastToWBP_UI_Tablet (Class|FGTaskTablet|GetWidget _returnvalue)))
    (Variables|Default|SetAs%20WBP%20UI%20Tablet _aswbp_ui_tablet))
  (if (== (Variables|Default|GetAs%20WBP%20UI%20Tablet) 0)
    (Development|PrintText "Could not get tablet" true true "(R=1.000000,G=0.000000,B=0.028078,A=1.000000)"))
  (return (Variables|Default|GetAs%20WBP%20UI%20Tablet)))