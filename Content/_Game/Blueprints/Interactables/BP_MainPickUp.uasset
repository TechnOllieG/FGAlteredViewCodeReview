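; Physics pickup actor, apparently a base for interactables, with optional distance culling and impact feedback.
; A looping one-second timer, started after a random delay to stagger instances, toggles mesh visibility by player distance.
; Hit notifications are enabled shortly after spawn; strong impacts play an FMOD sound, gated by a cooldown.
; After that cooldown, a randomly scaled decal spawns for static mesh hits if simulated velocity times mass exceeds a threshold.
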(event Custom|PickupCulling
  (bind _mesh (Variables|Character|GetMesh))
  ;[1 1 1] Pickup distance culling
  (if (Variables|Default|GetUseDistanceCulling)
    (Math|Float|CompareFloat (Transformation|GetDistanceTo (Game|Player|GetPlayerPawn 0)) (Variables|Default|GetPuckup%20Culling%20Distance)
      (:>
        (Rendering|SetVisibility _mesh false false))
      (:<
        (Rendering|SetVisibility _mesh true false)))))

(event EventBeginPlay
  (Utilities|FlowControl|Delay (Math|Random|RandomFloat))
  (Utilities|Time|SetTimerbyEvent (delegate Custom|PickupCulling) 1.0 true)
  (Utilities|FlowControl|Delay 2.0)
  (Class|PrimitiveComponent|SetNotifyRigidBodyCollision (Variables|Character|GetMesh) true))

(event Collision|EventHit
  (params (MyComp :type Primitive%20Component%20Object%20Reference) (Other :type Actor%20Object%20Reference) (OtherComp :type Primitive%20Component%20Object%20Reference) (bSelfMoved :type Boolean) (HitLocation :type Vector :default "0, 0, 0") (HitNormal :type Vector :default "0, 0, 0") (NormalImpulse :type Vector :default "0, 0, 0") (Hit :type Hit%20Result%20Structure%20%28by%20ref%29))
  (if (Variables|Default|GetOff%20Cooldown)
    (if (> (Math|Vector|VectorLength NormalImpulse) (Variables|Default|GetImpact%20Threshold))
      (Class|FMODBlueprintStatics|PlayEventatLocation (Variables|Default|GetFMOD%20Event) (Math|Conversions|ToTransform(Vector) HitLocation))
      (Variables|Default|SetOff%20Cooldown false)
      (Utilities|FlowControl|Delay (Variables|Default|GetCooldown%20Time))
      (Variables|Default|SetOff%20Cooldown true)
      ;[1 1 1] Impact decal spawner
      (if (Class|SceneComponent|IsAnySimulatingPhysics (Variables|Character|GetMesh))
        (if (Variables|Default|GetCan%20Leave%20Decal)
          (Utilities|Casting|CastToStaticMeshActor Other)
          (Math|Float|CompareFloat (* (Math|Vector|VectorLength (Transformation|GetVelocity)) (Physics|GetMass (Variables|Character|GetMesh))) (Variables|Default|GetDecal%20Force%20Treshold)
            (:>
              (Game|SpawnActorfromClass "/Game/_Game/Blueprints/BP_ImpactDecal.BP_ImpactDecal_C" (Math|Transform|MakeTransform HitLocation (Transformation|GetActorRotation) (* (Transformation|GetActorScale3D) (Math|Random|RandomFloatinRange 0.5 1.0))) "Undefined" 0 0))))))))

(fn ConstructionScript)