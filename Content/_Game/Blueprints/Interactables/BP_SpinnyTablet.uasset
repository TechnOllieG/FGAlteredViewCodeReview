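; Interactable tablet that flashes blue, green, red and yellow emissive pieces when used.
; On BeginPlay it binds to its child actor FGInteractable's OnInteract and sets that actor's mesh collision to BlockAll.
; Each enabled color pulses the Emissive parameter of a dynamic material made in the construction script.
; Pulses run in parallel through latent delays, with NoDelay choosing the color that lights immediately while the others wait TimeDelay.
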(event Custom|OnInteract_Event_0
  (params (Interactable :type FG%20Interactable%20Object%20Reference))
  (Utilities|FlowControl|Sequence
    (:then_0
      (if (Variables|Default|GetBlueColor)
        (if (== (Variables|Default|GetNoDelay) 4)
          _
          (else
            (Utilities|FlowControl|Delay (Variables|Default|GetTimeDelay))))
        (Rendering|Material|SetScalarParameterValue (Variables|Default|GetDynamicMatBlue) "Emissive" 2e+01 :!class /Script/Engine.MaterialInstanceDynamic)
        (Utilities|FlowControl|Delay (Variables|Default|GetTimeDelay))
        (Rendering|Material|SetScalarParameterValue (Variables|Default|GetDynamicMatBlue) "Emissive" 0.0 :!class /Script/Engine.MaterialInstanceDynamic)))
    (:then_1
      (if (Variables|Default|GetGreenColor)
        (if (== (Variables|Default|GetNoDelay) 3)
          _
          (else
            (Utilities|FlowControl|Delay (Variables|Default|GetTimeDelay))))
        (Rendering|Material|SetScalarParameterValue (Variables|Default|GetDynamicMatGreen) "Emissive" 2e+01 :!class /Script/Engine.MaterialInstanceDynamic)
        (Utilities|FlowControl|Delay (Variables|Default|GetTimeDelay))
        (Rendering|Material|SetScalarParameterValue (Variables|Default|GetDynamicMatGreen) "Emissive" 0.0 :!class /Script/Engine.MaterialInstanceDynamic)))
    (:then_2
      (if (Variables|Default|GetRedColor)
        (if (== (Variables|Default|GetNoDelay) 2)
          _
          (else
            (Utilities|FlowControl|Delay (Variables|Default|GetTimeDelay))))
        (Rendering|Material|SetScalarParameterValue (Variables|Default|GetDynamicMatRed) "Emissive" 2e+01 :!class /Script/Engine.MaterialInstanceDynamic)
        (Utilities|FlowControl|Delay (Variables|Default|GetTimeDelay))
        (Rendering|Material|SetScalarParameterValue (Variables|Default|GetDynamicMatRed) "Emissive" 0.0 :!class /Script/Engine.MaterialInstanceDynamic)))
    (:then_3
      (if (Variables|Default|GetYellowColor)
        (if (== (Variables|Default|GetNoDelay) 1)
          _
          (else
            (Utilities|FlowControl|Delay (Variables|Default|GetTimeDelay))))
        (Rendering|Material|SetScalarParameterValue (Variables|Default|GetDynamicMatYellow) "Emissive" 2e+01 :!class /Script/Engine.MaterialInstanceDynamic)
        (Utilities|FlowControl|Delay (Variables|Default|GetTimeDelay))
        (Rendering|Material|SetScalarParameterValue (Variables|Default|GetDynamicMatYellow) "Emissive" 0.0 :!class /Script/Engine.MaterialInstanceDynamic)))))

(event EventBeginPlay
  (bind _asfginteractable (Utilities|Casting|CastToFGInteractable (Variables|/Script/Engine.ChildActorComponent|GetChildActor (Variables|Default|GetChildActor))))
  (EventDispatchers|AssignOnInteract _asfginteractable (delegate Custom|OnInteract_Event_0))
  (Collision|SetCollisionProfileName (Actor|GetComponentbyClass _asfginteractable "/Script/Engine.StaticMeshComponent") "BlockAll" true :!class /Script/Engine.PrimitiveComponent))

(event Collision|EventActorBeginOverlap
  (params (OtherActor :type Actor%20Object%20Reference)))

(event EventTick
  (params (DeltaSeconds :type Float%20%28single-precision%29)))

(fn ConstructionScript
  (bind _returnvalue (Rendering|Material|CreateDynamicMaterialInstance (Variables|Default|GetBlue) 0 0 "None" :!class /Script/Engine.PrimitiveComponent))
  (Variables|Default|SetDynamicMatBlue _returnvalue)
  (bind _returnvalue_2 (Rendering|Material|CreateDynamicMaterialInstance (Variables|Default|GetGreen) 0 0 "None" :!class /Script/Engine.PrimitiveComponent))
  (Variables|Default|SetDynamicMatGreen _returnvalue_2)
  (bind _returnvalue_3 (Rendering|Material|CreateDynamicMaterialInstance (Variables|Default|GetRed) 0 0 "None" :!class /Script/Engine.PrimitiveComponent))
  (Variables|Default|SetDynamicMatRed _returnvalue_3)
  (bind _returnvalue_4 (Rendering|Material|CreateDynamicMaterialInstance (Variables|Default|GetYellow) 0 0 "None" :!class /Script/Engine.PrimitiveComponent))
  (Variables|Default|SetDynamicMatYellow _returnvalue_4))