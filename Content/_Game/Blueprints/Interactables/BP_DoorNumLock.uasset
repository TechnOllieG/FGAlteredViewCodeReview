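; Sliding double door with a lock, opened through the OpenDoor event, which completes its task component once open.
; BeginPlay caches both panels' closed positions and computes their X slide targets.
; OpenDoor spins the lock on one timeline, then plays a sound and lerps the panels apart on a second.
; Flags gate it to open only, with no close path; Interact and ScanKeyCard are empty.
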(event EventBeginPlay
  ;[1 1 1] Comment
  (Variables|Default|SetUnlocked true)
  (Variables|Default|SetbIsOpen true)
  (bind _output_get (Variables|Default|SetRightDoorVector (Variables|/Script/Engine.SceneComponent|GetRelativeLocation (Variables|Default|GetRightDoor))))
  (Variables|Default|SetMaxRightDoorVector (Math|Vector|MakeVector (+ (Variables|Default|GetMaxSlideDistanceRight) (.x _output_get)) (.y _output_get) (.z _output_get)))
  (bind _output_get_2 (Variables|Default|SetLeftDoorVector (Variables|/Script/Engine.SceneComponent|GetRelativeLocation (Variables|Default|GetLeftDoor))))
  (Variables|Default|SetMaxLeftDoorVector (Math|Vector|MakeVector (+ (Variables|Default|GetMaxSlideDistanceLeft) (.x _output_get_2)) (.y _output_get_2) (.z _output_get_2)))
  (Components|Timeline|SetTimelineLength (Variables|Default|GetTimeline_0) (Variables|Default|GetTimeToOpenClose)))

(event Collision|EventActorBeginOverlap
  (params (OtherActor :type Actor%20Object%20Reference)))

(event EventTick
  (params (DeltaSeconds :type Float%20%28single-precision%29)))

(event EventInteract
  ;[1 1 1] OpenDoor
)

(event EventOpenDoor
  ;[1 1 1] OpenDoor
  (if (Variables|Default|GetFinished)
    (Variables|Default|SetFinished false)
    (if (Variables|Default|GetbIsOpen)
      (Variables|Default|SetbIsOpen false)
      (Variables|Default|SetClosedOpenInt 1)
      (Timeline|Timeline_1 Play
        (:Update
          (Transformation|AddRelativeRotation (Variables|Default|GetLock) (Math|Rotator|Lerp(Rotator) "0, 0, 0" (Variables|Default|GetB) (Utilities|Time|GetWorldDeltaSeconds)) false false))
        (:Finished
          (Class|FMODBlueprintStatics|PlayEvent2D "/Game/FMOD/Events/Mechanisms/Door_Sci-Fi.Door_Sci-Fi")
          (Timeline|Timeline_0 Play
            (:Update
              (bind _output_get (Variables|Default|SetCurrentTime (Math|Float|Clamp(Float) (+ (Variables|Default|GetCurrentTime) (* (Variables|Default|GetClosedOpenInt) (Utilities|Time|GetWorldDeltaSeconds))) 0.0 (Variables|Default|GetTimeToOpenClose))))
              (Development|PrintString (Utilities|String|ToString(Float) _output_get) true true "(R=0.000000,G=0.660000,B=1.000000,A=1.000000)" 1e+02)
              (Transformation|SetRelativeLocation (Variables|Default|GetLeftDoor) (Math|Vector|Lerp(Vector) (Variables|Default|GetLeftDoorVector) (Variables|Default|GetMaxLeftDoorVector) (Math|Float|Clamp(Float) (/ (Variables|Default|GetCurrentTime) (Variables|Default|GetTimeToOpenClose)))) false false)
              (Transformation|SetRelativeLocation (Variables|Default|GetRightDoor) (Math|Vector|Lerp(Vector) (Variables|Default|GetRightDoorVector) (Variables|Default|GetMaxRightDoorVector) (Math|Float|Clamp(Float) (/ (Variables|Default|GetCurrentTime) (Variables|Default|GetTimeToOpenClose)))) false false))
            (:Finished
              (Variables|Default|SetFinished false)
              (Class|FGTaskComponent|CompleteTaskComponent (Variables|Default|GetTaskComponent)))))))))

(event EventScanKeyCard
  ;[1 1 1] OpenDoor
)

(fn ConstructionScript)