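; BP_NumPadForDoor is an interactable number pad, named as a door control, whose own logic here only supplies its press sound.
; InteractSound plays the Button_Press audio event at the actor's location, gated by a successful cast of the game mode to BP_GameMode.
; The construction script only calls the parent, and BeginPlay, overlap and Tick are disabled stubs.
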(event EventBeginPlay
  (|CallParentFunction) ; This node is disabled and will not be called.\nDrag off pins to build functionality.
)

(event Collision|EventActorBeginOverlap
  (params (OtherActor :type Actor%20Object%20Reference))
  (|CallParentFunction OtherActor) ; This node is disabled and will not be called.\nDrag off pins to build functionality.
)

(event EventTick
  (params (DeltaSeconds :type Float%20%28single-precision%29))
  (|CallParentFunction DeltaSeconds) ; This node is disabled and will not be called.\nDrag off pins to build functionality.
)

(event EventInteractSound
  (Utilities|Casting|CastToBP_GameMode (Game|GetGameMode))
  (Class|FMODBlueprintStatics|PlayEventatLocation "/Game/FMOD/Events/Interactables/Button_Press.Button_Press" (Math|Conversions|ToTransform(Vector) (Transformation|GetActorLocation))))

(fn ConstructionScript
  (|CallParentFunction))