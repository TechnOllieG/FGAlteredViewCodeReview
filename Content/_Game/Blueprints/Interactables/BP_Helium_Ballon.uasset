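; Interactable helium balloon that floats on a physics thruster and can be popped.
; A looping timer re-aligns the thruster to a fixed world rotation so its thrust direction holds as the balloon moves.
; A hit above a speed threshold spawns a randomly scaled stain decal and destroys only the mesh component, without sound.
; Interacting instead plays the pop audio event and destroys the whole actor, leaving no decal.
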(event Custom|Physics%20Tick
  (Transformation|SetWorldRotation (Variables|Default|GetPhysicsThruster) "-90.000000,-0.000000, 0" false false))

(event EventInteract
  (Utilities|Casting|CastToBP_GameMode (Game|GetGameMode))
  (Class|FMODBlueprintStatics|PlayEventatLocation "/Game/FMOD/Events/Interactables/Balloon_Pop.Balloon_Pop" (Math|Conversions|ToTransform(Vector) (Transformation|GetActorLocation)))
  (Actor|DestroyActor))

(event Collision|EventHit
  (params (MyComp :type Primitive%20Component%20Object%20Reference) (Other :type Actor%20Object%20Reference) (OtherComp :type Primitive%20Component%20Object%20Reference) (bSelfMoved :type Boolean) (HitLocation :type Vector :default "0, 0, 0") (HitNormal :type Vector :default "0, 0, 0") (NormalImpulse :type Vector :default "0, 0, 0") (Hit :type Hit%20Result%20Structure%20%28by%20ref%29))
  (Math|Float|CompareFloat (Math|Vector|VectorLength (Transformation|GetComponentVelocity (Variables|Default|GetSM_Balloon))) (Variables|Default|GetPop%20Treshold)
    (:>
      (Game|SpawnActorfromClass "/Game/_Game/Blueprints/BP_BalloonStainDecal.BP_BalloonStainDecal_C" (Math|Transform|MakeTransform (Transformation|GetActorLocation) "0, 0, 0" (* (Transformation|GetActorScale3D) (Math|Random|RandomFloatinRange 0.5 1.0))) "Undefined" 0 0)
      (Components|DestroyComponent (Variables|Default|GetSM_Balloon)))))

(event EventBeginPlay
  (Utilities|Time|SetTimerbyEvent (delegate Custom|Physics%20Tick) 0.2 true))

(fn ConstructionScript)