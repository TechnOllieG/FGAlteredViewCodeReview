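; Card-scanner sliding double door that toggles open and closed on ScanKeyCard or OpenDoor, with sound and Niagara reader feedback.
; BeginPlay caches closed and maximum slide positions; opening spins the lock via LockTimeline, then runs OpenTimeLine.
; The timeline clocks a signed, clamped time accumulator that lerps both panels, reversing to close, while a Finished flag blocks re-triggering.
; IsOpen reads inverted, starting true while the panels are at their closed positions.
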(event EventBeginPlay
  (Niagara|SetNiagaraVariable(LinearColor) (Variables|Default|GetCardreaderVFX) "False Color_Color" (Variables|Default|GetCardScanColor))
  (Variables|Default|SetbIsOpen true)
  (bind _output_get (Variables|Default|SetRightDoorVector (Variables|/Script/Engine.SceneComponent|GetRelativeLocation (Variables|Default|GetSM_Door_Right))))
  (Variables|Default|SetMaxRightDoorVector (Math|Vector|MakeVector (+ (Variables|Default|GetMaxSlideDistanceRight) (.x _output_get)) (.y _output_get) (.z _output_get)))
  (bind _output_get_2 (Variables|Default|SetLeftDoorVector (Variables|/Script/Engine.SceneComponent|GetRelativeLocation (Variables|Default|GetSM_Door_Left))))
  (Variables|Default|SetMaxLeftDoorVector (Math|Vector|MakeVector (+ (Variables|Default|GetMaxSlideDistanceLeft) (.x _output_get_2)) (.y _output_get_2) (.z _output_get_2)))
  (Components|Timeline|SetTimelineLength (Variables|Default|GetOpenTimeLine) (Variables|Default|GetTimeToOpenClose)))

(event Collision|EventActorBeginOverlap
  (params (OtherActor :type Actor%20Object%20Reference)))

(event EventTick
  (params (DeltaSeconds :type Float%20%28single-precision%29)))

(event EventInteract
  ;[1 1 1] OpenDoor
)

(event EventOpenDoor
  ;[1 1 1] OpenDoor
  (if (Variables|Default|GetFinished)
    (Variables|Default|SetFinished false)
    (if (Variables|Default|GetbIsOpen)
      (Variables|Default|SetbIsOpen false)
      (Variables|Default|SetClosedOpenInt 1)
      (Timeline|LockTimeline Play
        (:Update
          (Transformation|AddRelativeRotation (Variables|Default|GetSM_Door_Lock) (Math|Rotator|Lerp(Rotator) "0, 0, 0" (Variables|Default|GetB) (Utilities|Time|GetWorldDeltaSeconds)) false false))
        (:Finished
          (Class|FMODBlueprintStatics|PlayEvent2D "/Game/FMOD/Events/Mechanisms/Door_Sci-Fi.Door_Sci-Fi")
          (Timeline|OpenTimeLine Play
            (:Update
              (Variables|Default|SetCurrentTime (Math|Float|Clamp(Float) (+ (Variables|Default|GetCurrentTime) (* (Variables|Default|GetClosedOpenInt) (Utilities|Time|GetWorldDeltaSeconds))) 0.0 (Variables|Default|GetTimeToOpenClose)))
              (Transformation|SetRelativeLocation (Variables|Default|GetSM_Door_Left) (Math|Vector|Lerp(Vector) (Variables|Default|GetLeftDoorVector) (Variables|Default|GetMaxLeftDoorVector) (Math|Float|Clamp(Float) (/ (Variables|Default|GetCurrentTime) (Variables|Default|GetTimeToOpenClose)))) false false)
              (Transformation|SetRelativeLocation (Variables|Default|GetSM_Door_Right) (Math|Vector|Lerp(Vector) (Variables|Default|GetRightDoorVector) (Variables|Default|GetMaxRightDoorVector) (Math|Float|Clamp(Float) (/ (Variables|Default|GetCurrentTime) (Variables|Default|GetTimeToOpenClose)))) false false)
              (Class|NiagaraComponent|SetVariableBool (Variables|Default|GetCardreaderVFX) "AccessGranted" true))
            (:Finished
              (Variables|Default|SetFinished true)))))
      (else
        (Variables|Default|SetbIsOpen true)
        (Variables|Default|SetClosedOpenInt -1)
        (Class|FMODBlueprintStatics|PlayEvent2D "/Game/FMOD/Events/Mechanisms/Door_Sci-Fi.Door_Sci-Fi")
        (Timeline|OpenTimeLine Reverse)))))

(event EventScanKeyCard
  ;[1 1 1] OpenDoor
  (Class|FMODBlueprintStatics|PlayEvent2D "/Game/FMOD/Events/Mechanisms/Keycard_Reader.Keycard_Reader")
  (if (Variables|Default|GetFinished)
    (Variables|Default|SetFinished false)
    (if (Variables|Default|GetbIsOpen)
      (Variables|Default|SetbIsOpen false)
      (Variables|Default|SetClosedOpenInt 1)
      (Timeline|LockTimeline Play
        (:Update
          (Transformation|AddRelativeRotation (Variables|Default|GetSM_Door_Lock) (Math|Rotator|Lerp(Rotator) "0, 0, 0" (Variables|Default|GetB) (Utilities|Time|GetWorldDeltaSeconds)) false false))
        (:Finished
          (Class|FMODBlueprintStatics|PlayEvent2D "/Game/FMOD/Events/Mechanisms/Door_Sci-Fi.Door_Sci-Fi")
          (Timeline|OpenTimeLine Play
            (:Update
              (Variables|Default|SetCurrentTime (Math|Float|Clamp(Float) (+ (Variables|Default|GetCurrentTime) (* (Variables|Default|GetClosedOpenInt) (Utilities|Time|GetWorldDeltaSeconds))) 0.0 (Variables|Default|GetTimeToOpenClose)))
              (Transformation|SetRelativeLocation (Variables|Default|GetSM_Door_Left) (Math|Vector|Lerp(Vector) (Variables|Default|GetLeftDoorVector) (Variables|Default|GetMaxLeftDoorVector) (Math|Float|Clamp(Float) (/ (Variables|Default|GetCurrentTime) (Variables|Default|GetTimeToOpenClose)))) false false)
              (Transformation|SetRelativeLocation (Variables|Default|GetSM_Door_Right) (Math|Vector|Lerp(Vector) (Variables|Default|GetRightDoorVector) (Variables|Default|GetMaxRightDoorVector) (Math|Float|Clamp(Float) (/ (Variables|Default|GetCurrentTime) (Variables|Default|GetTimeToOpenClose)))) false false)
              (Class|NiagaraComponent|SetVariableBool (Variables|Default|GetCardreaderVFX) "AccessGranted" true))
            (:Finished
              (Variables|Default|SetFinished true)))))
      (else
        (Variables|Default|SetbIsOpen true)
        (Variables|Default|SetClosedOpenInt -1)
        (Class|FMODBlueprintStatics|PlayEvent2D "/Game/FMOD/Events/Mechanisms/Door_Sci-Fi.Door_Sci-Fi")
        (Timeline|OpenTimeLine Reverse)))))

(fn ConstructionScript)