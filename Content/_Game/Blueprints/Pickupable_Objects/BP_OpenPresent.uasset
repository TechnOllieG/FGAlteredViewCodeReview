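; BP_OpenPresent is a pickupable-object present that, when interacted with, opens into a new actor and removes itself.
; Interact enables its collision, waits briefly, then spawns an actor of RobotReference's class at the Spawn component's transform.
; It then releases both cable ends on the referenced helium balloon and destroys itself, which only happens if the balloon cast succeeds.
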(event EventInteract
  (Collision|SetActorEnableCollision true)
  (Utilities|FlowControl|Delay 0.2)
  (Game|SpawnActorfromClass (Utilities|GetClass (Variables|Default|GetRobotReference)) (Transformation|GetWorldTransform (Variables|Default|GetSpawn)) "Undefined" 0 0)
  (bind _asbp_helium_ballon_with_string (Utilities|Casting|CastToBP_Helium_BallonWithString (Variables|Default|Getballonreference)))
  (Variables|/Script/CableComponent.CableComponent|SetbAttachEnd (Variables|/Game/_Game/Blueprints/Interactables/BP_Helium_BallonWithString.BP_Helium_BallonWithString_C|GetCable _asbp_helium_ballon_with_string) false)
  (Variables|/Script/CableComponent.CableComponent|SetbAttachStart (Variables|/Game/_Game/Blueprints/Interactables/BP_Helium_BallonWithString.BP_Helium_BallonWithString_C|GetCable _asbp_helium_ballon_with_string) false)
  (Actor|DestroyActor))

(fn ConstructionScript)