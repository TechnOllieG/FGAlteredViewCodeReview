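; Pickupable red pencil cup that can be filled with coffee and spills it on a hard impact.
; FillWithCoffee shows the coffee plane and sets the Coffee flag, while BeginPlay turns off CanLeaveDecal.
; While physics-simulated, a hit on a StaticMeshActor with speed times mass above the spill threshold spawns a randomly scaled coffee decal, then empties the cup.
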(event EventBeginPlay
  (|CallParentFunction)
  (Variables|Default|SetCan%20Leave%20Decal false))

(event Collision|EventHit
  (params (MyComp :type Primitive%20Component%20Object%20Reference) (Other :type Actor%20Object%20Reference) (OtherComp :type Primitive%20Component%20Object%20Reference) (bSelfMoved :type Boolean) (HitLocation :type Vector :default "0, 0, 0") (HitNormal :type Vector :default "0, 0, 0") (NormalImpulse :type Vector :default "0, 0, 0") (Hit :type Hit%20Result%20Structure%20%28by%20ref%29))
  (|CallParentFunction MyComp Other OtherComp bSelfMoved HitLocation HitNormal NormalImpulse Hit)
  ;[1 1 1] Coffee Spill
  (if (Class|SceneComponent|IsAnySimulatingPhysics (Variables|Character|GetMesh))
    (if (Variables|Default|GetCoffee)
      (Utilities|Casting|CastToStaticMeshActor Other)
      (Math|Float|CompareFloat (* (Math|Vector|VectorLength (Transformation|GetVelocity)) (Physics|GetMass (Variables|Character|GetMesh))) (Variables|Default|GetSpill%20Force%20Treshold)
        (:>
          (Game|SpawnActorfromClass "/Game/_Game/Blueprints/BP_ImpactDecal_Coffee.BP_ImpactDecal_Coffee_C" (Math|Transform|MakeTransform HitLocation (Transformation|GetActorRotation) (* (Transformation|GetActorScale3D) (Math|Random|RandomFloatinRange 0.5 1.0))) "Undefined" 0 0)
          (Variables|Default|SetCoffee false)
          (Rendering|SetVisibility (Variables|Default|GetCoffeePlane) false false))))))

(fn ConstructionScript)

(fn FillwithCoffee
  (|CallParentFunction)
  (Rendering|SetVisibility (Variables|Default|GetCoffeePlane) true false)
  (Variables|Default|SetCoffee true))