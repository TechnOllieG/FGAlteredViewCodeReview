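; Pickupable pencil holder that can be filled with coffee and spills it on hard impacts.
; FillWithCoffee, overriding the parent, sets IsFull and shows the coffee plane, which a looping timer eases toward its fill height.
; While simulating physics, hits against static mesh actors compare speed times mass to a threshold; exceeding it empties the holder, hides the plane and spawns a randomly scaled coffee decal.
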(event Custom|Fill%20Coffee
  (bind _coffeeplane (Variables|Default|GetCoffeePlane))
  (bind _returnvalue (Transformation|GetRelativeTransform _coffeeplane))
  (if (Variables|Default|GetIsFull)
    (Transformation|SetRelativeLocation _coffeeplane (Math|Vector|MakeVector (.x (.location _returnvalue)) (.y (.location _returnvalue)) (Math|Float|Lerp (.z (.location _returnvalue)) (Variables|Default|GetCoffee%20Height) 0.1)) false false)))

(event EventBeginPlay
  (|CallParentFunction)
  (Utilities|Time|SetTimerbyEvent (delegate Custom|Fill%20Coffee) 0.1 true))

(event Collision|EventHit
  (params (MyComp :type Primitive%20Component%20Object%20Reference) (Other :type Actor%20Object%20Reference) (OtherComp :type Primitive%20Component%20Object%20Reference) (bSelfMoved :type Boolean) (HitLocation :type Vector :default "0, 0, 0") (HitNormal :type Vector :default "0, 0, 0") (NormalImpulse :type Vector :default "0, 0, 0") (Hit :type Hit%20Result%20Structure%20%28by%20ref%29))
  (|CallParentFunction MyComp Other OtherComp bSelfMoved HitLocation HitNormal NormalImpulse Hit)
  (if (Class|SceneComponent|IsAnySimulatingPhysics (Variables|Character|GetMesh))
    (Utilities|Casting|CastToStaticMeshActor Other)
    (if (Variables|Default|GetIsFull)
      (Math|Float|CompareFloat (* (Math|Vector|VectorLength (Transformation|GetVelocity)) (Physics|GetMass (Variables|Character|GetMesh))) (Variables|Default|GetSpill%20Force%20Treshold)
        (:>
          (Game|SpawnActorfromClass "/Game/_Game/Blueprints/BP_ImpactDecal_Coffee.BP_ImpactDecal_Coffee_C" (Math|Transform|MakeTransform HitLocation (Transformation|GetActorRotation) (* (Transformation|GetActorScale3D) (Math|Random|RandomFloatinRange 0.5 1.0))) "Undefined" 0 0)
          (Variables|Default|SetIsFull false)
          (Rendering|SetVisibility (Variables|Default|GetCoffeePlane) false false))))))

(fn ConstructionScript)

(fn FillwithCoffee
  (|CallParentFunction)
  (Variables|Default|SetIsFull true)
  (Rendering|SetVisibility (Variables|Default|GetCoffeePlane) true false))